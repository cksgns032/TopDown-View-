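; BP_ItemBase is an item actor that configures itself as either an owned item or a world drop.
; On BeginPlay it adds a mouse-point tag, looks up its equip location and rotation in DT_Equipe_Pos by item ID, and applies its mesh.
; With an owner, it hides the name widget and makes its box ignore Visibility traces.
; Without one, it adds an overlay material and shows the item name.
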(event EventBeginPlay
  (Utilities|Array|Add (Variables|Actor|GetTags) (Utilities|Name|EnumtoName (Utilities|Enum|LiteralenumBP_EMousePoint "NewEnumerator2")))
  (bind _outrownames (DataTable|GetDataTableRowNames "/Game/1_BluePrint/DataTable/DT_Equipe_Pos.DT_Equipe_Pos"))
  (bind _array_element (Utilities|Array|ForEachLoopwithBreak _outrownames :!label _label)
    (:LoopBody
      (bind _returnvalue (Utilities|GetDataTableRow "/Game/1_BluePrint/DataTable/DT_Equipe_Pos.DT_Equipe_Pos" _array_element)
        (:then
          (if (== (.ItemID (Utilities|Struct|BreakBPStruct_EquipePos _returnvalue)) (.uniqueid (Variables|Default|GetItemData)))
            (Variables|Default|SetEquip_Location (.Location (Utilities|Struct|BreakBPStruct_EquipePos _returnvalue)))
            (Variables|Default|SetEquip_Rotation (.Rotator (Utilities|Struct|BreakBPStruct_EquipePos _returnvalue)))
            (goto _label Break)))))
    (:Completed
      (Components|StaticMesh|SetStaticMesh (Variables|Default|GetStaticMesh) (.mesh (Variables|Default|GetItemData)))
      (Utilities|IsValid (Components|GetOwner)
        (:Is%20Valid
          (Rendering|SetVisibility (Variables|Default|GetWidget) false false)
          (Collision|SetCollisionResponsetoChannel (Variables|Default|GetBox) "ECC_Visibility" "ECR_Ignore"))
        (:Is%20Not%20Valid
          (Rendering|Material|SetOverlayMaterial (Actor|GetComponentbyClass "/Script/Engine.StaticMeshComponent") "/Game/6_Material/PostProcessMaterial.PostProcessMaterial" :!class /Script/Engine.MeshComponent)
          (Rendering|SetVisibility (Variables|Default|GetWidget) true false)
          (bind _aswbp_drop_item_name (Utilities|Casting|CastToWBP_DropItemName (UserInterface|GetWidget (Variables|Default|GetWidget))))
          (Default|SetName _aswbp_drop_item_name (.name (Variables|Default|GetItemData))))))))

(event Collision|EventActorBeginOverlap
  (params (OtherActor :type Actor%20Object%20Reference)))

(event EventTick
  (params (DeltaSeconds :type Float%20%28single-precision%29)))

(fn ConstructionScript)
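; Combo attack component for the player character that attacks the enemy under the mouse cursor.
; Attack picks a montage through Chooser evaluation switched on equipped item ID, then either moves toward an out-of-range enemy or turns, stops and plays it.
; The range check is 2D and allows for the enemy's hitbox extent.
; AddCombo increments the count and reopens attacking, while montage blend-out resets the combo a tick later.
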(event Custom|Attack
  (bind _self self)
  ;[0.15 0.15 0.15 0.5] 공격 가능 체크
  (if (Variables|Default|GetbCanAttack)
    (Variables|Default|SetbCanAttack false)
    (Variables|Default|SetbIsAttack true)
    (bind _asbp_game_instance (Utilities|Casting|CastToBP_GameInstance (Game|GetGameInstance)))
    (bind _return_value (Default|GetEquipData _asbp_game_instance (Variables|/Game/1_BluePrint/BP_GameInstance.BP_GameInstance_C|GetEquipSlot _asbp_game_instance)))
    (switch int (.uniqueid _return_value)
      (:Default
        (bind _result (|EvaluateChooser2 _self)
          (:execute
            (Variables|Default|SetMontage%20to%20Play _result))))
      (:0
        (bind _result_2 (|EvaluateChooser2 _self)
          (:execute
            (Variables|Default|SetMontage%20to%20Play _result_2))))
      (:1
        (bind _result_3 (|EvaluateChooser2 _self)
          (:execute
            (Variables|Default|SetMontage%20to%20Play _result_3)))))
    (bind _as캐릭터 (Utilities|Casting|CastToCharacter (Components|GetOwner)))
    (bind _output_get (Variables|Default|SetCharacter _as캐릭터))
    (bind _as플레이어_컨트롤러 (Utilities|Casting|CastToPlayerController (Pawn|GetController _output_get)))
    (bind _output_get_2 (Variables|Default|SetPlayerController _as플레이어_컨트롤러))
    (if (.bBlockingHit (Collision|BreakHitResult (.HitResult (Game|Player|GetHitResultUnderCursorbyChannel _output_get_2 "TraceTypeQuery1" true))))
      (bind _asbp_enemy (Utilities|Casting|CastToBP_Enemy (.HitActor (Collision|BreakHitResult (.HitResult (Game|Player|GetHitResultUnderCursorbyChannel _output_get_2 "TraceTypeQuery1" true))))))
      (bind (_return_value_2 _return_vector) (CallFunction|DistanceCheck (Transformation|GetActorLocation (.HitActor (Collision|BreakHitResult (.HitResult (Game|Player|GetHitResultUnderCursorbyChannel _output_get_2 "TraceTypeQuery1" true))))) (Math|Vector|VectorLength (Math|Vector|MakeVector (.X (Math|Vector|BreakVector (Components|Box|GetScaledBoxExtent (Variables|/Game/1_BluePrint/Monster/BP_Enemy.BP_Enemy_C|GetHitBox _asbp_enemy)))) (.Y (Math|Vector|BreakVector (Components|Box|GetScaledBoxExtent (Variables|/Game/1_BluePrint/Monster/BP_Enemy.BP_Enemy_C|GetHitBox _asbp_enemy)))) 0.0))))
      (if _return_value_2
        (AI|Navigation|SimpleMovetoLocation (Variables|Default|GetPlayerController) _return_vector)
        (Variables|Default|SetbCanAttack true)
        (Variables|Default|SetbIsAttack false)
        (else
          (CallFunction|LookTarget (Transformation|GetActorLocation (.HitActor (Collision|BreakHitResult (.HitResult (Game|Player|GetHitResultUnderCursorbyChannel _output_get_2 "TraceTypeQuery1" true))))))
          (AI|Navigation|StopMovement (Variables|Default|GetPlayerController))
          (Animation|Montage|PlayMontage (Actor|GetComponentbyClass (Components|GetOwner) "/Script/Engine.SkeletalMeshComponent") (Variables|Default|GetMontage%20to%20Play)
            (:OnBlendOut
              (Utilities|FlowControl|DelayUntilNextTick)
              (CallFunction|ResetCombo)))))
      (else
        (Variables|Default|SetbCanAttack true)
        (Variables|Default|SetbIsAttack false)))))

(event Custom|LookTarget
  (params (TargetLocation :type Vector))
  (Transformation|SetActorRotation (Variables|Default|GetCharacter) (Math|Rotator|MakeRotator 0.0 0.0 (.Yaw (Math|Rotator|BreakRotator (Math|Rotator|FindLookatRotation (Transformation|GetActorLocation (Variables|Default|GetCharacter)) TargetLocation))))))

(event EventBeginPlay)

(event EventTick
  (params (DeltaSeconds :type Float%20%28single-precision%29)))

(fn AddCombo
  (Math|Integer|IncrementInt (Variables|Default|GetComboCount)
    (:%20%20
      (Variables|Default|SetbCanAttack true)
      (Variables|Default|SetbIsAttack false))))

(fn ResetCombo
  (Variables|Default|SetComboCount 0)
  (Variables|Default|SetbCanAttack true)
  (Variables|Default|SetbIsAttack false))

(fn DistanceCheck
  (params (TargetCenter :type Vector) (HitBoxSize :type Float%20%28double-precision%29))
  (bind _character (Variables|Default|GetCharacter))
  (bind _returnvalue (Transformation|GetActorLocation _character))
  (return (> (- (Math|Vector|Distance2D(Vector) _returnvalue TargetCenter) HitBoxSize) (Variables|Default|GetAttackRange)) (- TargetCenter (* (Math|Vector|Normalize (- TargetCenter _returnvalue)) (- (Variables|Default|GetAttackRange) (+ (Components|Capsule|GetScaledCapsuleRadius (Variables|/Script/Engine.Character|GetCapsuleComponent (Variables|Default|GetCharacter))) (Variables|Default|GetDistanceSpace)))))))
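; Gameplay ability for a montage-driven attack that spawns a hit box on an animation event.
; AttackMontage supplies an enemy owner's first attack montage; the top-down character branch returns no montage.
; A one-shot gameplay event wait spawns BP_HitBox at the owner's transform and runs its box trace.
; Montage blend-out, interruption or cancellation destroys the hit box and ends the ability.
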(event Ability|EventActivateAbility
  (bind _returnvalue (Ability|GetOwningActorfromActorInfo))
  (|PlayMontageandWaitProxy "None" (CallFunction|AttackMontage) 1.0 "None" true 1.0 0.0 false
    (:then
      (Ability|Async|WaitGameplayEventToActor _returnvalue "(TagName=\"AnimEvent\")" true
        (:EventReceived
          (bind _returnvalue_2 (Game|SpawnActorfromClass "/Game/1_BluePrint/BP_HitBox.BP_HitBox_C" (Transformation|GetActorTransform _returnvalue) "Undefined" "MultiplyWithRoot" _returnvalue (Variables|/Script/Engine.Actor|GetInstigator _returnvalue)))
          (bind _output_get (Variables|Default|SetHit%20Box _returnvalue_2))
          (Class|HitBox|DoBoxTrace _output_get "100.000000,100.000000,100.000000" 0.0))))
    (:OnBlendOut
      (Actor|DestroyActor (Variables|Default|GetHit%20Box) :!label _label)
      (Ability|EndAbility))
    (:OnInterrupted
      (goto _label))
    (:OnCancelled
      (goto _label))))

(event Ability|EventOnEndAbility
  (params (bWasCancelled :type Boolean)))

(fn AttackMontage
  (bind _returnvalue (Ability|GetOwningActorfromActorInfo))
  (bind _asbp_top_down_character (Utilities|Casting|CastToBP_TopDownCharacter _returnvalue)
    (:then
      (Utilities|IsValid _asbp_top_down_character
        (:Is%20Valid
          (return 0))
        (:Is%20Not%20Valid
          _)))
    (:CastFailed
      _))
  (bind _asbp_enemy (Utilities|Casting|CastToBP_Enemy _returnvalue)
    (:then
      (return (Utilities|Array|Get(acopy) (Variables|/Script/TopViewGame.BaseMonster|GetAttackMontages _asbp_enemy))))
    (:CastFailed
      (return 0))))
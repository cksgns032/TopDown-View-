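; BP_Enemy is a monster that tags itself with a mouse-point enum name, takes damage, dies and drops a weapon.
; AnyDamage lowers HP, updates the HP and damage-text widgets, then plays a hit or death montage while flagging IsHit.
; After the death montage blends out, it disables collision, stops AI movement and behavior, and runs a timeline-driven dissolve material.
; When the dissolve finishes, it spawns a random DropItems entry and destroys itself.
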(event Custom|DropItem
  (Game|SpawnActorfromClass (Utilities|Array|Get(acopy) (Variables|Default|GetDropItems) (Math|Random|RandomIntegerinRange 0 (- (Utilities|Array|Length (Variables|Default|GetDropItems)) 0))) (Math|Transform|MakeTransform (Transformation|GetActorLocation) "90.000000,0.000000,0.000000" "1.000000,1.000000,1.000000") "Undefined" "MultiplyWithRoot" 0 0))

(event Collision|EventActorBeginOverlap
  (params (OtherActor :type Actor%20Object%20Reference)))

(event EventTick
  (params (DeltaSeconds :type Float%20%28single-precision%29)))

(event Game|Damage|EventAnyDamage
  (params (Damage :type Float%20%28single-precision%29) (DamageType :type Damage%20Type%20Object%20Reference) (InstigatedBy :type Controller%20Object%20Reference) (DamageCauser :type Actor%20Object%20Reference))
  (bind _mesh (Variables|Character|GetMesh))
  (bind _mesh_2 (Variables|Character|GetMesh))
  (Variables|Default|SetCurHp (Math|Integer|Max(Integer) (Math|Float|Round (- (Variables|Default|GetCurHp) Damage))))
  (CallFunction|UpdateHp)
  (CallFunction|ShowDamage (Math|Float|Truncate Damage))
  (if (> (Variables|Default|GetCurHp) 0)
    (Animation|Montage|PlayMontage _mesh (Variables|Default|GetHitMontage) 1.0 0.0 "Default"
      (:then
        (Variables|Default|SetbIsHit true)
        (Development|PrintString "Hit"))
      (:OnBlendOut
        (Variables|Default|SetbIsHit false)
        (Development|PrintString "Completed")))
    (else
      (Animation|Montage|PlayMontage _mesh (Variables|Default|GetDeadMontage) 1.0 0.0 "Default"
        (:then
          (Variables|Default|SetbIsHit true))
        (:OnBlendOut
          (Utilities|FlowControl|Sequence
            (:then_0
              (Variables|Default|SetbIsHit false))
            (:then_1
              ;[0.15 0.15 0.15 0.5] 기능 비활성화
              (Collision|SetCollisionEnabled (Variables|Collision|GetCapsuleComponent) "NoCollision")
              (Collision|SetCollisionEnabled (Variables|Character|GetMesh) "NoCollision")
              (Collision|SetCollisionEnabled (Variables|Default|GetHitBox) "NoCollision")
              (AI|Navigation|StopMovement (AI|GetAIController self)))
            (:then_2
              ;[0.15 0.15 0.15 0.5] 몽타주 실행
              (Class|SkeletalMeshComponent|SetEnableAnimation _mesh_2 false)
              (bind _returnvalue (Rendering|Material|CreateDynamicMaterialInstance _mesh_2 0 "/Game/6_Material/DessolveMaterial.DessolveMaterial" "None" :!class /Script/Engine.PrimitiveComponent))
              (Rendering|Material|SetTextureParameterValue _returnvalue "Param" (Variables|Default|GetTexture))
              (bind _asbp_monster_controller (Utilities|Casting|CastToBP_MonsterController (AI|GetAIController self)))
              (Default|StopBehavior _asbp_monster_controller)
              (bind _dessolvecurve (Timeline|DessolveTimeline Play)
                (:Update
                  (Rendering|Material|SetScalarParameterValue _returnvalue "Dissolve" _dessolvecurve :!class /Script/Engine.MaterialInstanceDynamic))
                (:Finished
                  (CallFunction|DropItem)
                  (Actor|DestroyActor))))))))))

(event EventBeginPlay
  (Utilities|Array|Add (Variables|Actor|GetTags) (Utilities|Name|EnumtoName (Utilities|Enum|LiteralenumBP_EMousePoint "NewEnumerator1")))
  (Variables|Default|SetCurHp (Variables|Default|GetMaxHp))
  (CallFunction|UpdateHp)
  (Utilities|Array|Add (Variables|Default|GetDropItems) "/Game/1_BluePrint/Actor/BP_OneHandSword.BP_OneHandSword_C")
  (Utilities|Array|Add (Variables|Default|GetDropItems) "/Game/1_BluePrint/Actor/BP_TwoHandSword.BP_TwoHandSword_C"))

(fn ConstructionScript)

(fn UpdateHp
  (bind _aswbp_hp (Utilities|Casting|CastToWBP_HP (UserInterface|GetWidget (Variables|Default|GetWidget_HP))))
  (Default|UpdateHp _aswbp_hp (Variables|Default|GetCurHp) (Variables|Default|GetMaxHp)))

(fn ShowDamage
  (params (Damage :type Integer))
  (bind _aswbp_damage_text (Utilities|Casting|CastToWBP_DamageText (UserInterface|GetWidget (Variables|Default|GetWidget_Damage))))
  (Default|ShowDamage _aswbp_damage_text Damage))